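; Window manager Blueprint that shows paged text windows, such as dialogue or messages, and pauses the game while one is open.
; BeginPlay creates the TestHUD widget; OpenWindow adds it to the viewport, plays a sound and fills its three text fields from a TestDataTable row.
; Each row's NextID chains pages: the Decide input shows the next row, or closes the window and unpauses at "-1".
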(event `self.ReceiveBeginPlay`
  (bind _returnvalue (`|CreateWidget` "/Game/MyData/BluePrints/TextWindow/TestHUD.TestHUD_C"))
  (set `self.WindowWidget` _returnvalue))

(event `self.ReceiveTick`
  (params (DeltaSeconds :type "Float (single-precision)")))

(event `InputAction|Decide` :consume false :paused true
  (params (Key :type "Key Structure"))
  (bind _nextid (`self.nextID`))
  (:`Pressed`
    (if (== _nextid "-1") :!pinned true
      (`self.CloseWindow`)
      (else
        (`self.SetText` _nextid)))))

(fn `CloseWindow`
  (bind _windowwidget (`self.WindowWidget`))
  (if (`Widget.IsVisible` _windowwidget)
    (`Widget.RemoveFromParent` _windowwidget)
    (`GameplayStatics.SetGamePaused` false)))

(fn `OpenWindow`
  (params (TextID :type Name))
  (bind _windowwidget (`self.WindowWidget`))
  (if (not (`Widget.IsVisible` _windowwidget))
    (`UserWidget.AddToViewport` _windowwidget 0)
    (`self.SetText` TextID)
    (`GameplayStatics.PlaySound2D` "/Engine/EditorSounds/GamePreview/EndSimulate.EndSimulate" 1.0 1.0 0.0 null null)
    (`GameplayStatics.SetGamePaused` true)))

(fn `SetText`
  (params (textID :type Name))
  (bind _windowwidget (`self.WindowWidget`))
  (bind _returnvalue (`|GetDataTableRow` "/Game/MyData/BluePrints/TextWindow/TestDataTable.TestDataTable" textID)
    (:`then`
      (bind (_text1 _text2 _text3 _nextid) (break `/Game/MyData/BluePrints/TextWindow/test` _returnvalue))
      (set `/Game/MyData/BluePrints/TextWindow/TestHUD.text1` _text1 _windowwidget)
      (set `/Game/MyData/BluePrints/TextWindow/TestHUD.text2` _text2 _windowwidget)
      (set `/Game/MyData/BluePrints/TextWindow/TestHUD.text3` _text3 _windowwidget)
      (set `self.nextID` _nextid))))

(fn `UserConstructionScript`)