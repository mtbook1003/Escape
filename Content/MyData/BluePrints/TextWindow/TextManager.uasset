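; TextManager is an actor that shows paged text windows and pauses the game while one is open.
; BeginPlay copies TextDataTable rows into an array, creating the WindowHUD widget inside that loop.
; OpenWindow shows an entry by array index, and the Decide input follows each NextID until -1 closes the window.
; CloseWindow clears the text, unpauses and disables input, while the EnableInput call in OpenWindow is unconnected.
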(event `self.ReceiveBeginPlay`
  (bind _outrownames (`DataTableFunctionLibrary.GetDataTableRowNames` "/Game/MyData/BluePrints/TextWindow/TextDataTable.TextDataTable")) ; データテーブルから行の名前を取得
  (for _array_element _outrownames
    ;[1 1 1] データがある間、取得を続ける
    (bind _returnvalue (`|GetDataTableRow` "/Game/MyData/BluePrints/TextWindow/TextDataTable.TextDataTable" _array_element) ; 一致する名前のデータを探す(ここ気持ち悪い)
      (:`then`
        (`KismetArrayLibrary.Array_Add` (`self.textData`) _returnvalue) ; 配列にデータを追加
        (bind _returnvalue_2 (`|CreateWidget` "/Game/MyData/BluePrints/TextWindow/WindowHUD.WindowHUD_C"))
        (set `self.windowHUD` _returnvalue_2)))))

(event `InputAction|Decide` :paused true
  (params (Key :type "Key Structure"))
  (bind (_name _text01 _text02 _text03 _nextid) (break `/Game/MyData/BluePrints/TextWindow/TextData` (`self.nowTextData`)))
  (:`Pressed`
    (if (`self.isOpenWindow`)
      (if (== _nextid -1)
        (`self.CloseWindow`)
        (else
          (bind _textdata (`self.GetNextTextData` _nextid))
          (`self.SetText` _textdata)
          (set `self.nowTextData` _textdata))))))

(event `self.ReceiveTick`
  (params (DeltaSeconds :type "Float (single-precision)")))

(fn `CloseWindow`
  (bind _windowhud (`self.windowHUD`))
  (set `/Game/MyData/BluePrints/TextWindow/WindowHUD.text01` "" _windowhud)
  (set `/Game/MyData/BluePrints/TextWindow/WindowHUD.text02` "" _windowhud)
  (set `/Game/MyData/BluePrints/TextWindow/WindowHUD.text03` "" _windowhud)
  (`Widget.RemoveFromParent` _windowhud)
  (set `self.isOpenWindow` false)
  (`self.DisableInput` (`GameplayStatics.GetPlayerController` 0))
  (`GameplayStatics.SetGamePaused` false))

(fn `GetNextTextData`
  (params (TextID :type Integer))
  (returns (TextData :type "/Game/MyData/BluePrints/TextWindow/TextData Structure"))
  (if (and (>= TextID 0) (<= TextID (`KismetArrayLibrary.Array_LastIndex` (`self.textData`))))
    (return (`|GetArrayItem` (`self.textData`) TextID))))

(fn `OpenWindow`
  (params (textID :type Integer))
  (bind _windowhud (`self.windowHUD`))
  (if (`self.isOpenWindow`)
    _
    (elif (and (>= textID 0) (<= textID (`KismetArrayLibrary.Array_LastIndex` (`self.textData`))))
      (`UserWidget.AddToViewport` _windowhud 0)
      (set `self.windowHUD` _windowhud)
      (bind _textdata (`self.GetNextTextData` textID))
      (`self.SetText` _textdata)
      (set `self.nowTextData` _textdata)
      (set `self.isOpenWindow` true)
      (`GameplayStatics.SetGamePaused` true))))

(fn `SetText`
  (params (textData :type "/Game/MyData/BluePrints/TextWindow/TextData Structure"))
  (bind (_name _text01 _text02 _text03) (break `/Game/MyData/BluePrints/TextWindow/TextData` textData))
  (bind _windowhud (`self.windowHUD`))
  (set `/Game/MyData/BluePrints/TextWindow/WindowHUD.text01` _text01 _windowhud)
  (set `/Game/MyData/BluePrints/TextWindow/WindowHUD.text02` _text02 _windowhud)
  (set `/Game/MyData/BluePrints/TextWindow/WindowHUD.text03` _text03 _windowhud))

(fn `UserConstructionScript`)