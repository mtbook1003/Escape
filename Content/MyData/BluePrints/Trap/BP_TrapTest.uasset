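; BP_TrapTest is a test trap trigger that shows a text window and starts a bush event when the player walks into its box.
; On overlap by MyPlayer, it opens a TextID window through the WindowManager on MyGameModeBase, then calls the StartEventBush dispatcher.
; Leftover calls to an Event reference for move requests and rock movement are unwired and never run.
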(event `self.Box.OnComponentBeginOverlap`
  (params (OverlappedComponent :type "PrimitiveComponent Object Reference") (OtherActor :type "Actor Object Reference") (OtherComp :type "PrimitiveComponent Object Reference") (OtherBodyIndex :type Integer) (bFromSweep :type Boolean) (SweepResult :type "HitResult Structure (by ref)"))
  (cast `/Game/MyData/BluePrints/MyPlayer` OtherActor)
  (bind _asmy_game_mode_base (cast `/Game/MyData/BluePrints/MyGameModeBase` (`GameplayStatics.GetGameMode`)))
  (`/Game/MyData/BluePrints/TextWindow/WindowManager.OpenWindow` (`/Game/MyData/BluePrints/MyGameModeBase.WindowManager` _asmy_game_mode_base) (`self.textID`))
  (`self.StartEvent_Bush`))

(fn `UserConstructionScript`)