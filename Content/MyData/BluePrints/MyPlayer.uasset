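; Player Blueprint that moves and looks around from axis inputs and hits objects in front of it on the Decide action.
; Movement follows the camera's forward and right vectors, turn and look axes drive controller yaw and pitch, and BeginPlay applies an initial pitch input.
; Decide calls CheckWindowActor, which runs a short forward capsule multi-trace on Visibility and sends ApplyDamage to the first valid hit actor.
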(event `self.ReceiveBeginPlay`
  (`self.AddControllerPitchInput` 10.0))

(event `InputAction|Decide` :consume false
  (params (Key :type "Key Structure"))
  (:`Pressed`
    (`self.CheckWindowActor`)))

(event `self.ReceiveTick`
  (params (DeltaSeconds :type "Float (single-precision)")))

(event `InputAxis|MoveRight`
  (params (AxisValue :type "Float (single-precision)"))
  (`self.AddMovementInput` (`SceneComponent.GetRightVector` (`self.Camera`)) AxisValue))

(event `InputAxis|MoveForward`
  (params (AxisValue :type "Float (single-precision)"))
  (`self.AddMovementInput` (`SceneComponent.GetForwardVector` (`self.Camera`)) AxisValue))

(event `InputAxis|TurnRate`
  (params (AxisValue :type "Float (single-precision)"))
  (`self.AddControllerYawInput` AxisValue))

(event `InputAxis|LookUpRate`
  (params (AxisValue :type "Float (single-precision)"))
  (`self.AddControllerPitchInput` AxisValue))

(fn `CheckWindowActor`
  (bind _returnvalue (`self.K2_GetActorLocation`))
  (bind _outhits (`KismetSystemLibrary.CapsuleTraceMulti` _returnvalue (+ _returnvalue (* (`self.GetActorForwardVector`) 100.0)) 10.0 50.0 "TraceTypeQuery1"))
  (for _array_element _outhits
    (bind (_bblockinghit _binitialoverlap _time _distance _location _impactpoint _normal _impactnormal _physmat _hitactor) (`GameplayStatics.BreakHitResult` _array_element))
    (`/Engine/EditorBlueprintResources/StandardMacros.IsValid` _hitactor
      (:`Is Valid`
        (`GameplayStatics.ApplyDamage` _hitactor 1.0)
        (break)))))

(fn `UserConstructionScript`)