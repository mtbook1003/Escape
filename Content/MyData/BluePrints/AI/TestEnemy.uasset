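; Test enemy actor that checks every tick whether a player is directly in front of it.
; CanSeePlayerPawn casts a single line trace along the forward vector for a configurable sight length, drawn as a one-frame debug line.
; It returns the hit actor if tagged "Player", but Tick does not use the result, so detection triggers no behavior yet.
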(event `self.ReceiveTick`
  (params (DeltaSeconds :type "Float (single-precision)"))
  (`self.CanSeePlayerPawn`))

(fn `CanSeePlayerPawn`
  (returns (Player :type "Actor Object Reference"))
  (bind _returnvalue (`self.K2_GetActorLocation`))
  (bind _outhit (`KismetSystemLibrary.LineTraceSingle` :`Start` _returnvalue :`End` (+ _returnvalue (* (`self.GetActorForwardVector`) (`self.ShightLength`))) :`TraceChannel` "TraceTypeQuery3" :`DrawDebugType` "ForOneFrame"))
  (bind (_bblockinghit _binitialoverlap _time _distance _location _impactpoint _normal _impactnormal _physmat _hitactor) (`GameplayStatics.BreakHitResult` _outhit))
  (if (`KismetSystemLibrary.IsValid` _hitactor)
    (if (`self.ActorHasTag` _hitactor "Player")
      (return _hitactor))))

(fn `UserConstructionScript`)