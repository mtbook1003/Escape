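; AI controller for TestEnemy that sets up patrolling along the pawn's patrol points.
; On BeginPlay it caches those points, initializes BlackboardTestEnemy with the pawn's wait time and runs the BP_Patrol behavior tree.
; A separate AIMoveTo event cycles through the points with a wrapping index, re-arming itself by timer only on success.
; Nothing in this graph initially triggers that event.
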(event `self.ReceiveBeginPlay`
  (bind _astest_enemy (cast `/Game/MyData/BluePrints/AI/TestEnemy` (`self.K2_GetPawn`)))
  (set `self.TargetPoint` (`/Game/MyData/BluePrints/AI/TestEnemy.PatrolPoint` _astest_enemy))
  (`self.UseBlackboard` "/Game/MyData/BluePrints/AI/BlackboardTestEnemy.BlackboardTestEnemy")
  (`BlackboardComponent.SetValueAsFloat` (`self.Blackboard`) "WaitTime" (`/Game/MyData/BluePrints/AI/TestEnemy.WaitTime` _astest_enemy))
  (`self.RunBehaviorTree` "/Game/MyData/BluePrints/AI/BP_Patrol.BP_Patrol"))

(event `GoToTargetPoint_Event`
  (`|AIMoveTo` (`self.K2_GetPawn`) (`self.GetDestination`) null
    (:`OnSuccess`
      (`self.AddNextPoint`)
      (`KismetSystemLibrary.K2_SetTimerDelegate` (delegate `GoToTargetPoint_Event`) 0.1))))

(fn `AddNextPoint`
  (set `self.nextID` (mod (+ (`self.nextID`) 1) (`KismetArrayLibrary.Array_Length` (`self.TargetPoint`)))))

(fn `GetDestination`
  (returns (ReturnValue :type "Vector Structure"))
  (return (`self.K2_GetActorLocation` (`|GetArrayItem` (`self.TargetPoint`) (`self.nextID`)))))

(fn `UserConstructionScript`)