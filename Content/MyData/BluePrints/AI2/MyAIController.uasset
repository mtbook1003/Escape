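; AI controller that makes an Enemy pawn patrol endlessly through its assigned patrol points.
; On BeginPlay it casts the controlled pawn to Enemy and copies that pawn's PatrolPoint array.
; GoToNext moves the pawn to the current point with AIMoveTo, then on success advances the index with modulo wrap-around and calls itself again.
; A failed move is not handled, so the patrol stops there.
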(event `self.ReceiveBeginPlay`
  (bind _asenemy (cast `/Game/MyData/BluePrints/AI2/Enemy` (`self.K2_GetPawn`)))
  (set `self.PatrolPoint` (`/Game/MyData/BluePrints/AI2/Enemy.PatrolPoint` _asenemy))
  (`self.GoToNext`))

(event `GoToNext`
  (`|AIMoveTo` (`self.K2_GetPawn`) (0.0 0.0 0.0) (`|GetArrayItem` (`self.PatrolPoint`) (`self.NextIndex`))
    (:`OnSuccess`
      (`self.CalcNextIndex`)
      (`self.GoToNext`))))

(fn `CalcNextIndex`
  (set `self.NextIndex` (mod (+ (`self.NextIndex`) 1) (`KismetArrayLibrary.Array_Length` (`self.PatrolPoint`)))))

(fn `UserConstructionScript`)